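; Wolf AI ("Loup") that hunts the sheep herd (Troupeau_Mouton) and makes a single attack.
; PawnSensing sighting starts a one-time AIMoveTo toward the herd.
; The first sphere overlap with the herd, gated by DoOnce, cuts its sheep count and walk speed, then zeroes the wolf's walk speed.
; AddMoutons, not called here, increments the wolf's own sheep count and derives walk speed from it.
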(event OnSeePawn(PawnSensing)
  (params (Pawn :type Pawn%20Object%20Reference))
  (bind _astroupeau_mouton (Utilities|Casting|CastToTroupeau_Mouton Pawn))
  (Utilities|FlowControl|DoOnce false
    (:Completed
      (AI|AIMoveTo self "0, 0, 0" _astroupeau_mouton 5.0 false))))

(event OnComponentBeginOverlap(Sphere)
  (params (OverlappedComponent :type Primitive%20Component%20Object%20Reference) (OtherActor :type Actor%20Object%20Reference) (OtherComp :type Primitive%20Component%20Object%20Reference) (OtherBodyIndex :type Integer) (bFromSweep :type Boolean) (SweepResult :type Hit%20Result%20Structure%20%28by%20ref%29))
  (bind _astroupeau_mouton (Utilities|Casting|CastToTroupeau_Mouton OtherActor))
  (Utilities|FlowControl|DoOnce false
    (:Completed
      (Variables|/Game/Blueprints/Character/Troupeau_Mouton.Troupeau_Mouton_C|SetNbMoutons _astroupeau_mouton (- (Variables|/Game/Blueprints/Character/Troupeau_Mouton.Troupeau_Mouton_C|GetNbMoutons _astroupeau_mouton) 3.0))
      (Variables|/Game/Blueprints/Character/Troupeau_Mouton.Troupeau_Mouton_C|SetMax%20Walk%20Speed _astroupeau_mouton (- (Variables|/Game/Blueprints/Character/Troupeau_Mouton.Troupeau_Mouton_C|GetMax%20Walk%20Speed _astroupeau_mouton) 6e+02))
      (Development|PrintString (Utilities|String|ToString(Float) (Variables|/Game/Blueprints/Character/Troupeau_Mouton.Troupeau_Mouton_C|GetNbMoutons _astroupeau_mouton)))
      (Variables|Default|SetMax%20Walk%20Speed 0.0))))

(event EventBeginPlay)

(fn ConstructionScript)

(fn AddMoutons
  (Variables|Default|SetNbMoutons (+ (Variables|Default|GetNbMoutons) 1.0))
  (Variables|Default|SetMax%20Walk%20Speed (+ (* (- (Variables|Default|GetNbMoutons) 1.0) 2e+02) 1.2e+03))
  (Development|PrintString (Utilities|String|ToString(Float) (Variables|Default|GetMax%20Walk%20Speed))))