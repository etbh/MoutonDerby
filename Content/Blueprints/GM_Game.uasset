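; Game mode that times a sheep-based round and shows the UI_TimerTest end screen.
; StartGame opens a gate that lets Tick accumulate delta seconds into Time, and Ending closes it after passing Time to the widget.
; Ending shows the cursor and switches input to UI only.
; Tick also creates that screen, without passing Time, on every frame while NumberSheep is zero or less.
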(event Custom|Ending
  (bind _returnvalue (Game|GetPlayerController 0))
  (Utilities|FlowControl|Sequence
    (:then_0
      (Variables|/Script/Engine.PlayerController|SetbShowMouseCursor _returnvalue true)
      (bind _returnvalue_2 (UserInterface|CreateWidget "/Game/Blueprints/UI_TimerTest.UI_TimerTest_C" _returnvalue))
      (Default|AddTime _returnvalue_2 (Variables|Default|GetTime))
      (UserInterface|Viewport|AddtoViewport _returnvalue_2 0)
      (Input|SetInputModeUIOnly _returnvalue _returnvalue_2 "DoNotLock"))
    (:then_1
      (Utilities|FlowControl|Gate true) ; enters at Close
    )))

(event Custom|StartGame
  (Utilities|FlowControl|Gate true) ; enters at Open
)

(event EventTick
  (params (DeltaSeconds :type Float%20%28single-precision%29))
  (bind _returnvalue (Game|GetPlayerController 0))
  (Utilities|FlowControl|Sequence
    (:then_0
      (Utilities|FlowControl|Gate true
        (:Exit
          (Variables|Default|SetTime (+ DeltaSeconds (Variables|Default|GetTime))))))
    (:then_1
      ;[1 1 1] Timer
      (if (<= (Variables|Default|GetNumberSheep) 0)
        (Variables|/Script/Engine.PlayerController|SetbShowMouseCursor _returnvalue true)
        (bind _returnvalue_2 (UserInterface|CreateWidget "/Game/Blueprints/UI_TimerTest.UI_TimerTest_C" _returnvalue))
        (UserInterface|Viewport|AddtoViewport _returnvalue_2 0)
        (Input|SetInputModeUIOnly _returnvalue _returnvalue_2 "DoNotLock")))))

(event EventBeginPlay)

(fn ConstructionScript)