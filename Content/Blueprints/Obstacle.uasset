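; Obstacle actor that hurts the sheep of a herd (Troupeau_Mouton) on contact and wears out as it does.
; Each sheep entering its Box collision takes damage and costs the obstacle one point of Durability, and the actor destroys itself when that runs out.
; Disconnected nodes for creating a widget linked to the obstacle and adding it to the viewport remain in the graph but never run.
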(event OnComponentBeginOverlap(Box)
  (params (OverlappedComponent :type Primitive%20Component%20Object%20Reference) (OtherActor :type Actor%20Object%20Reference) (OtherComp :type Primitive%20Component%20Object%20Reference) (OtherBodyIndex :type Integer) (bFromSweep :type Boolean) (SweepResult :type Hit%20Result%20Structure%20%28by%20ref%29))
  ;[1 1 1] Begin Overlap
  (bind _astroupeau_mouton (Utilities|Casting|CastToTroupeau_Mouton OtherActor))
  (Default|TakeDamage _astroupeau_mouton)
  (bind _output_get (Variables|Default|SetDurability (- (Variables|Default|GetDurability) 1.0)))
  (if (<= _output_get 0.0)
    (Actor|DestroyActor self)))

(fn ConstructionScript)