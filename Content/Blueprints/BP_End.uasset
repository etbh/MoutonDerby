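; BP_End is an end-zone trigger that calls Ending on GM_Game when an actor overlaps its box.
; It then calls StopSheep if the overlapping actor is a Troupeau_Mouton.
; The CastToPlayer helper compares the actor's class to the default pawn and only prints a French debug message on mismatch.
; The construction script sizes the box from a Transform variable.
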(event OnComponentBeginOverlap(Box)
  (params (OverlappedComponent :type Primitive%20Component%20Object%20Reference) (OtherActor :type Actor%20Object%20Reference) (OtherComp :type Primitive%20Component%20Object%20Reference) (OtherBodyIndex :type Integer) (bFromSweep :type Boolean) (SweepResult :type Hit%20Result%20Structure%20%28by%20ref%29))
  (CallFunction|CasttoPlayer OtherActor)
  (bind _asgm_game (Utilities|Casting|CastToGM_Game (Game|GetGameMode)))
  (Default|Ending _asgm_game)
  (bind _astroupeau_mouton (Utilities|Casting|CastToTroupeau_Mouton OtherActor))
  (Default|StopSheep _astroupeau_mouton))

(fn ConstructionScript
  ;[1 1 1] select box transform
  (Components|Box|SetBoxExtent (Variables|Default|GetBox) (* (Variables|General|GetTransform) 1e+02) true))

(fn CasttoPlayer
  (params (Other%20Actor :type Actor%20Object%20Reference))
  (if (== (Utilities|GetClass Other%20Actor) (Variables|/Script/Engine.GameModeBase|GetDefaultPawnClass (Game|GetGameMode)))
    (return)
    (else
      (Development|PrintString "le cast n'a pas fonctioné"))))