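; Player character for a sheep herd in an auto-runner, moving forward on its own while the player strafes and steers with clamped yaw input.
; BeginPlay locks movement for a printed countdown, then enables input and starts the game through GM_Game.
; Tick applies the current max walk speed and drives forward movement.
; Adding sheep raises that speed, damage cuts sheep and speed, and both update the GameMode's count.
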(event Custom|TakeDamage
  ;[1 1 1] Take Damage
  (bind _output_get (Variables|Default|SetNbMoutons (- (Variables|Default|GetNbMoutons) 3.0)))
  (Variables|/Game/Blueprints/GM_Game.GM_Game_C|SetNumberSheep (Variables|Default|GetGameMode) (Math|Float|Truncate _output_get))
  (Variables|Default|SetMax%20Walk%20Speed (- (Variables|Default|GetMax%20Walk%20Speed) 6e+02)))

(event Custom|StopSheep
  ;[1 1 1] stop player
  (Input|DisableInput 0)
  (Variables|Default|SetCanMove? false))

(event EventTick
  (params (DeltaSeconds :type Float%20%28single-precision%29))
  (bind _charactermovement (Variables|Character|GetCharacterMovement))
  ;[1 1 1] Move Forward
  (if (Variables|Default|GetCanMove?)
    (Utilities|FlowControl|Sequence
      (:then_0
        (Variables|/Script/Engine.CharacterMovementComponent|SetMaxWalkSpeed _charactermovement (Variables|Default|GetMax%20Walk%20Speed)))
      (:then_1
        (Pawn|Input|AddMovementInput (Math|Vector|GetForwardVector (Math|Rotator|MakeRotator 0.0 0.0 (.yaw (Pawn|GetControlRotation :!class /Script/Engine.Pawn)))) (* DeltaSeconds (Variables|/Script/Engine.CharacterMovementComponent|GetMaxWalkSpeed _charactermovement)) false)))))

(event EventBeginPlay
  ;[1 1 1] Set GameMode
  (bind _asgm_game (Utilities|Casting|CastToGM_Game (Game|GetGameMode)))
  (Variables|Default|SetGameMode _asgm_game)
  (Input|DisableInput (Game|GetPlayerController 0))
  (Variables|Default|SetCanMove? false)
  (Utilities|FlowControl|Delay 2.0)
  (Development|PrintString "3")
  (Utilities|FlowControl|Delay 1.0)
  (Development|PrintString "2")
  (Utilities|FlowControl|Delay 1.0)
  (Development|PrintString "1")
  (Utilities|FlowControl|Delay 1.0)
  (Development|PrintString "Goooooooooooooooo !!!!!!!!!!!!!")
  (Input|EnableInput (Game|GetPlayerController 0))
  (Variables|Default|SetCanMove? true)
  (Default|StartGame (Variables|Default|GetGameMode)))

(event Input|AxisEvents|InputAxisRight/Left
  (params (AxisValue :type Float%20%28single-precision%29))
  ;[1 1 1] Move Right
  (Pawn|Input|AddMovementInput (Math|Vector|GetRightVector (Math|Rotator|MakeRotator 0.0 0.0 (.yaw (Pawn|GetControlRotation :!class /Script/Engine.Pawn)))) (* AxisValue (Variables|Default|GetR/Lspeed)) false))

(event Input|AxisEvents|InputAxisRotation
  (params (AxisValue :type Float%20%28single-precision%29))
  ;[1 1 1] Mouse Controller
  (Pawn|Input|AddControllerYawInput (Math|Float|Clamp(Float) AxisValue -0.5 0.5)))

(fn ConstructionScript)

(fn AddMoutons
  (bind _output_get (Variables|Default|SetNbMoutons (+ (Variables|Default|GetNbMoutons) 1.0)))
  (Variables|/Game/Blueprints/GM_Game.GM_Game_C|SetNumberSheep (Variables|Default|GetGameMode) (Math|Float|Truncate _output_get))
  (Variables|Default|SetMax%20Walk%20Speed (+ (* (- (Variables|Default|GetNbMoutons) 1.0) 2e+02) 1.2e+03))
  (Development|PrintString (Utilities|String|ToString(Float) (Variables|Default|GetMax%20Walk%20Speed))))